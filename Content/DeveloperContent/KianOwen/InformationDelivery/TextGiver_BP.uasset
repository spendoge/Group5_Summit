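; TextGiver_BP is a trigger actor that shows a message in the first-person player's HUD speech bubble.
; When the player character overlaps its collision box, it writes ColText into the SpeechBubbleMasterWBP text block and makes the bubble visible.
; After a Delay of Duration, it hides the bubble again, with no check for whether the player is still inside the box.
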(event `self.CollisionBox.OnComponentBeginOverlap`
  (params (OverlappedComponent :type "PrimitiveComponent Object Reference") (OtherActor :type "Actor Object Reference") (OtherComp :type "PrimitiveComponent Object Reference") (OtherBodyIndex :type Integer) (bFromSweep :type Boolean) (SweepResult :type "HitResult Structure (by ref)"))
  (bind _asbp_first_person_character (cast `/Game/StarterStuff/FirstPerson/Blueprints/BP_FirstPersonCharacter` OtherActor))
  (bind _speechbubblemaster_wbp (`/Game/DeveloperContent/CamiToye/Menu/PlayerHUD.SpeechBubbleMaster_WBP` (`/Game/StarterStuff/FirstPerson/Blueprints/BP_FirstPersonCharacter.PlayerHUD` _asbp_first_person_character)))
  (`TextBlock.SetText` (`/Game/DeveloperContent/KianOwen/InformationDelivery/SpeechBubbleMaster_WBP.TextBlock_44` _speechbubblemaster_wbp) (`KismetTextLibrary.Conv_StringToText` (`self.ColText`)))
  (`Widget.SetVisibility` _speechbubblemaster_wbp "Visible")
  (`KismetSystemLibrary.Delay` (`self.Duration`))
  (`Widget.SetVisibility` _speechbubblemaster_wbp "Hidden"))

(fn `UserConstructionScript`)