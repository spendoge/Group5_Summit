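; Trigger actor that shows a one-time speech bubble on the player's HUD when a first-person character overlaps it.
; It reveals InputText with a typewriter effect, appending characters to DisplayText through a short-delay loop and updating the bubble's text block.
; Once the full line is shown, it waits for Duration, then hides the bubble.
; The DoOnce gate precedes the character cast, so the first overlap by any actor uses up the trigger.
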(event `self.ReceiveActorBeginOverlap`
  (params (OtherActor :type "Actor Object Reference"))
  (`/Engine/EditorBlueprintResources/StandardMacros.DoOnce` false
    (:`Completed`
      (bind _asbp_first_person_character (cast `/Game/StarterStuff/FirstPerson/Blueprints/BP_FirstPersonCharacter` OtherActor))
      (bind _speechbubble_wbp (`/Game/DeveloperContent/CamiToye/Menu/PlayerHUD.SpeechBubble_WBP` (`/Game/StarterStuff/FirstPerson/Blueprints/BP_FirstPersonCharacter.PlayerHUD` _asbp_first_person_character)))
      (`Widget.SetVisibility` _speechbubble_wbp "Visible")
      (bind _array_element (`/Game/DeveloperContent/KianOwen/InformationDelivery/Loop.ForEachLoopDelay` (`KismetStringLibrary.GetCharacterArrayFromString` (`self.InputText`)) 0.01)
        (:`LoopBody`
          (bind _output_get (set `self.DisplayText` (`KismetStringLibrary.Concat_StrStr` (`self.DisplayText`) _array_element)))
          (`TextBlock.SetText` (`/Game/DeveloperContent/KianOwen/InformationDelivery/SpeechBubble_WBP.TextBlock_44` _speechbubble_wbp) (`KismetTextLibrary.Conv_StringToText` _output_get)))
        (:`Completed`
          (`KismetSystemLibrary.Delay` (`self.Duration`))
          (`Widget.SetVisibility` _speechbubble_wbp "Hidden"))))))

(fn `UserConstructionScript`)