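; BP_HintSIgn_Combined is a hint sign that reveals its glyphs and shows a text hint in the player's HUD speech bubble on interaction.
; A delayed for-each loop appends InputText's characters one at a time for a typewriter effect.
; The bubble hides after a configurable delay once typing ends, while the glyphs stay visible.
; A DoOnce with no reset limits the sign to a single use.
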(event `/Game/DeveloperContent/JacobStirling/Management/BI_Interaction.Interaction`
  (params (PlayerCharacter :type "/Game/StarterStuff/FirstPerson/Blueprints/BP_FirstPersonCharacter Object Reference"))
  (bind _speechbubble_wbp (`/Game/DeveloperContent/CamiToye/Menu/PlayerHUD.SpeechBubble_WBP` (`/Game/StarterStuff/FirstPerson/Blueprints/BP_FirstPersonCharacter.PlayerHUD` PlayerCharacter)))
  (`/Engine/EditorBlueprintResources/StandardMacros.DoOnce` false
    (:`Completed`
      (`SceneComponent.SetVisibility` (`self.Glyphs`) true false)
      (`Widget.SetVisibility` _speechbubble_wbp "Visible")
      (bind _array_element (`/Game/DeveloperContent/KianOwen/InformationDelivery/Loop.ForEachLoopDelay` (`KismetStringLibrary.GetCharacterArrayFromString` (`self.InputText`)) 0.01)
        (:`LoopBody`
          (bind _output_get (set `self.DisplayText` (`KismetStringLibrary.Concat_StrStr` (`self.DisplayText`) _array_element)))
          (`TextBlock.SetText` (`/Game/DeveloperContent/KianOwen/InformationDelivery/SpeechBubble_WBP.TextBlock_44` _speechbubble_wbp) (`KismetTextLibrary.Conv_StringToText` _output_get)))
        (:`Completed`
          (`KismetSystemLibrary.Delay` (`self.Duration`))
          (`Widget.SetVisibility` _speechbubble_wbp "Hidden"))))))

(fn `UserConstructionScript`)