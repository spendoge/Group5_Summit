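; A spike trap socket that raises and retracts a spike and hurts the player.
; Activate plays or reverses a timeline from its status flag, lerping the Cone between the NoSpike and YesSpike component locations; Deactivate reverses it from the current position.
; Overlap on the Damage component by the player character prints a message and applies fixed damage, with no check on spike state.
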(event `self.ReceiveBeginPlay`
  (`parent.ReceiveBeginPlay`)
  (set `self.Start Loc` (`SceneComponent.K2_GetComponentLocation` (`self.Cone`))))

(event `/Game/DeveloperContent/JacobStirling/Management/BI_SocketConnectors.Activate`
  (params (ActivityStatus :type Boolean))
  (if ActivityStatus
    (bind (_direction _newtrack_0) (`Timeline|Timeline_0` :!via `PlayFromStart` :!label _label)
      (:`Update`
        (`SceneComponent.K2_SetWorldLocation` (`self.Cone`) (`KismetMathLibrary.VLerp` (`SceneComponent.K2_GetComponentLocation` (`self.NoSpike`)) (`SceneComponent.K2_GetComponentLocation` (`self.YesSpike`)) _newtrack_0) false false)))
    (else
      (goto _label :!via `ReverseFromEnd`))))

(event `/Game/DeveloperContent/JacobStirling/Management/BI_SocketConnectors.Deactivate`
  (goto _label :!via `Reverse`))

(event `self.Damage.OnComponentBeginOverlap`
  (params (OverlappedComponent :type "PrimitiveComponent Object Reference") (OtherActor :type "Actor Object Reference") (OtherComp :type "PrimitiveComponent Object Reference") (OtherBodyIndex :type Integer) (bFromSweep :type Boolean) (SweepResult :type "HitResult Structure (by ref)"))
  (if (== OtherActor (`GameplayStatics.GetPlayerCharacter` 0))
    (`KismetSystemLibrary.PrintString` "Ouch")
    (`GameplayStatics.ApplyDamage` null 15.0)))

(fn `UserConstructionScript`
  (`parent.UserConstructionScript`))