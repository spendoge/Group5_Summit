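; Spike trap that lowers its spike once every connected pressure plate is pressed, and raises it when one is released afterward.
; Plate events shrink or refill the connected-plate array, and external Activate/Deactivate events drive the same logic.
; "Activate" means retract: a timeline moves the cone between marker positions while materials and Pusher collision switch.
; The damage overlap only prints "Ouch" for the player.
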(event `self.ReceiveBeginPlay`
  (bind _connectedpressureplates (`self.ConnectedPressurePlates`))
  (`parent.ReceiveBeginPlay`)
  (set `self.Start Loc` (`SceneComponent.K2_GetComponentLocation` (`self.Cone`)))
  ;[1 1 1] Bind events
  (add `/Game/DeveloperContent/JacobStirling/Actors/BP_PressurePlate.E_PressurePlateOverlapped` _connectedpressureplates (`|CreateDelegate` :!event `PressurePlateOverlapped`))
  (add `/Game/DeveloperContent/JacobStirling/Actors/BP_PressurePlate.E_PressurePlateNotOverlapped` _connectedpressureplates (`|CreateDelegate` :!event `PressurePlateNotOverlapped`)))

(event `DeactivateSpike`
  (`PrimitiveComponent.SetMaterial` (`self.Cone`) 0 "/Game/DeveloperContent/SpencerWright/Master_Materials/MI_SpikeOn.MI_SpikeOn" :!label _label)
  (`PrimitiveComponent.SetMaterial` (`self.Cube`) 0 "/Game/DeveloperContent/SpencerWright/Master_Materials/MI_SpikeOn.MI_SpikeOn")
  (`PrimitiveComponent.SetCollisionResponseToAllChannels` (`self.Pusher`) "ECR_Block")
  (bind (_direction _newtrack_0) (`Timeline|Timeline_0` :!via `PlayFromStart` :!label _label_2)
    (:`Update`
      (`SceneComponent.K2_SetWorldLocation` (`self.Cone`) (`KismetMathLibrary.VLerp` (`SceneComponent.K2_GetComponentLocation` (`self.NoSpike`)) (`SceneComponent.K2_GetComponentLocation` (`self.YesSpike`)) _newtrack_0) false false))))

(event `ActivateSpike`
  (params (Activity :type Boolean))
  (bind _output_get (set `self.Activity` Activity))
  (if _output_get
    (`PrimitiveComponent.SetMaterial` (`self.Cone`) 0 "/Game/DeveloperContent/SpencerWright/Master_Materials/MI_SpikeOff.MI_SpikeOff")
    (`PrimitiveComponent.SetMaterial` (`self.Cube`) 0 "/Game/DeveloperContent/SpencerWright/Master_Materials/MI_SpikeOff.MI_SpikeOff")
    (`PrimitiveComponent.SetCollisionResponseToAllChannels` (`self.Pusher`) "ECR_Ignore")
    (goto _label_2 :!via `ReverseFromEnd`)
    (else
      (goto _label))))

(event `/Game/DeveloperContent/JacobStirling/Management/BI_SocketConnectors.Activate`
  (params (ActivityStatus :type Boolean) (chargeLevel :type Integer))
  ;[1 1 1] Activate and Deactivate
  (`self.ActivateSpike` ActivityStatus))

(event `self.Damage.OnComponentBeginOverlap`
  (params (OverlappedComponent :type "PrimitiveComponent Object Reference") (OtherActor :type "Actor Object Reference") (OtherComp :type "PrimitiveComponent Object Reference") (OtherBodyIndex :type Integer) (bFromSweep :type Boolean) (SweepResult :type "HitResult Structure (by ref)"))
  (if (== OtherActor (`GameplayStatics.GetPlayerCharacter` 0))
    (`KismetSystemLibrary.PrintString` "Ouch")))

(event `/Game/DeveloperContent/JacobStirling/Management/BI_SocketConnectors.Deactivate`
  (params (chargeLevel :type Integer))
  ;[1 1 1] Activate and Deactivate
  (`self.DeactivateSpike`))

(fn `PressurePlateNotOverlapped`
  (params (PressurePlate :type "/Game/DeveloperContent/JacobStirling/Actors/BP_PressurePlate Object Reference"))
  (`KismetArrayLibrary.Array_Add` (`self.ConnectedPressurePlates`) PressurePlate)
  (if (`self.Activity`)
    (`self.DeactivateSpike`)))

(fn `PressurePlateOverlapped`
  (params (PressurePlate :type "/Game/DeveloperContent/JacobStirling/Actors/BP_PressurePlate Object Reference"))
  (bind _connectedpressureplates (`self.ConnectedPressurePlates`))
  (`KismetArrayLibrary.Array_RemoveItem` _connectedpressureplates PressurePlate)
  (if (<= (`KismetArrayLibrary.Array_Length` _connectedpressureplates) 0)
    (`self.ActivateSpike` true)))

(fn `UserConstructionScript`
  (`parent.UserConstructionScript`))