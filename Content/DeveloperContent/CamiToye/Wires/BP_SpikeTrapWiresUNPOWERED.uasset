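; Spike trap that extends or retracts through an Activate event, using a timeline to slide the cone while swapping on/off materials and toggling the Pusher's blocking collision.
; A Ball entering the Box retracts the spike and restarts a one-shot timer, with DebugDeactivate available to re-extend it.
; Player overlap with Damage only spawns a bleed effect and prints "Ouch", as the ApplyDamage call is unconnected.
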(event `self.ReceiveBeginPlay`
  (`parent.ReceiveBeginPlay`)
  (set `self.Start Loc` (`SceneComponent.K2_GetComponentLocation` (`self.Cone`))))

(event `self.Activate`
  (params (ActivityStatus :type Boolean) (chargeLevel :type Integer))
  (bind _pusher (`self.Pusher`))
  (if ActivityStatus
    (`PrimitiveComponent.SetMaterial` (`self.Cone`) 0 "/Game/DeveloperContent/SpencerWright/Master_Materials/MI_SpikeOn.MI_SpikeOn")
    (`PrimitiveComponent.SetMaterial` (`self.Cube`) 0 "/Game/DeveloperContent/SpencerWright/Master_Materials/MI_SpikeOn.MI_SpikeOn")
    (`PrimitiveComponent.SetCollisionResponseToAllChannels` _pusher "ECR_Block")
    (bind (_direction _newtrack_0) (`Timeline|Timeline_0` :!label _label)
      (:`Update`
        (`SceneComponent.K2_SetWorldLocation` (`self.Cone`) (`KismetMathLibrary.VLerp` (`SceneComponent.K2_GetComponentLocation` (`self.NoSpike`)) (`SceneComponent.K2_GetComponentLocation` (`self.YesSpike`)) _newtrack_0) false false)))
    (else
      (`PrimitiveComponent.SetMaterial` (`self.Cone`) 0 "/Game/DeveloperContent/SpencerWright/Master_Materials/MI_SpikeOff.MI_SpikeOff")
      (`PrimitiveComponent.SetMaterial` (`self.Cube`) 0 "/Game/DeveloperContent/SpencerWright/Master_Materials/MI_SpikeOff.MI_SpikeOff")
      (`PrimitiveComponent.SetCollisionResponseToAllChannels` _pusher "ECR_Ignore")
      (goto _label :!via `Reverse`))))

(event `self.Damage.OnComponentBeginOverlap`
  (params (OverlappedComponent :type "PrimitiveComponent Object Reference") (OtherActor :type "Actor Object Reference") (OtherComp :type "PrimitiveComponent Object Reference") (OtherBodyIndex :type Integer) (bFromSweep :type Boolean) (SweepResult :type "HitResult Structure (by ref)"))
  (bind _returnvalue (`GameplayStatics.GetPlayerCharacter` 0))
  (bind (_returnvalue_x _returnvalue_y _returnvalue_z) (`KismetMathLibrary.BreakVector` (`SceneComponent.K2_GetComponentLocation` (`Actor.RootComponent` (cast `/Game/StarterStuff/FirstPerson/Blueprints/BP_FirstPersonCharacter` _returnvalue :!pure true)))))
  (if (== OtherActor _returnvalue)
    (`NiagaraFunctionLibrary.SpawnSystemAtLocation` "/Game/DeveloperContent/CamiToye/Particles/Bleed.Bleed" (`KismetMathLibrary.MakeVector` _returnvalue_x _returnvalue_y (+ _returnvalue_z 85.0)))
    (`KismetSystemLibrary.PrintString` "Ouch")))

(event `self.Box.OnComponentBeginOverlap`
  (params (OverlappedComponent :type "PrimitiveComponent Object Reference") (OtherActor :type "Actor Object Reference") (OtherComp :type "PrimitiveComponent Object Reference") (OtherBodyIndex :type Integer) (bFromSweep :type Boolean) (SweepResult :type "HitResult Structure (by ref)"))
  (cast `/Game/DeveloperContent/CamiToye/Wires/Ball` OtherActor)
  (`self.Activate` false)
  (`KismetSystemLibrary.K2_ClearAndInvalidateTimerHandle` (`self.Timer`))
  (bind _returnvalue (`KismetSystemLibrary.K2_SetTimerDelegate` (`|CreateDelegate` :!event `DebugDeactivate`) (`self.Time`)))
  (set `self.Timer` _returnvalue))

(event `DebugDeactivate`
  (`self.Activate` true))

(fn `UserConstructionScript`
  (`parent.UserConstructionScript`))