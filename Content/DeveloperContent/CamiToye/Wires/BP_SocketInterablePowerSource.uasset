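; Powered ball emitter that repeatedly fires a Ball actor from its Arrow component while it has power.
; BeginPlay starts a looping timer that calls SpawnBall, storing the handle in StopFiring, which is not used afterward.
; Activate sets HasPower, which gates spawning while the timer keeps running.
; InLifeSpan serves as both the timer interval and a value passed to each spawned ball.
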(event `self.ReceiveBeginPlay`
  (bind _returnvalue (`KismetSystemLibrary.K2_SetTimerDelegate` (delegate `SpawnBall`) (`self.In Life Span`) true))
  (set `self.StopFiring` _returnvalue))

(event `SpawnBall`
  (if (`self.HasPower`)
    (`|SpawnActorFromClass` "/Game/DeveloperContent/CamiToye/Wires/Ball.Ball_C" (`SceneComponent.K2_GetComponentToWorld` (`self.Arrow`)) "Undefined" "OverrideRootScale" null (`self.In Life Span`) null)))

(event `/Game/DeveloperContent/JacobStirling/Management/BI_SocketConnectors.Activate`
  (params (ActivityStatus :type Boolean) (chargeLevel :type Integer))
  (set `self.HasPower` ActivityStatus))

(fn `UserConstructionScript`
  (`parent.UserConstructionScript`))