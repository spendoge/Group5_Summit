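; BP_WBC is a hazard with character movement that deals repeated damage to actors tagged Player inside its Box.
; Begin overlap starts a looping half-second timer that applies Damage to the overlapping actor.
; Any end overlap clears that timer, without checking which actor left.
; UpdateWalkSpeed sets the CharacterMovement max walk speed, but nothing in this Blueprint calls it.
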(event `self.Box.OnComponentEndOverlap`
  (params (OverlappedComponent :type "PrimitiveComponent Object Reference") (OtherActor :type "Actor Object Reference") (OtherComp :type "PrimitiveComponent Object Reference") (OtherBodyIndex :type Integer))
  ;[1 1 1] End Overlap
  (`KismetSystemLibrary.K2_ClearAndInvalidateTimerHandle` (`self.TimerHandle`)))

(event `self.Box.OnComponentBeginOverlap`
  (params (OverlappedComponent :type "PrimitiveComponent Object Reference") (OtherActor :type "Actor Object Reference") (OtherComp :type "PrimitiveComponent Object Reference") (OtherBodyIndex :type Integer) (bFromSweep :type Boolean) (SweepResult :type "HitResult Structure (by ref)"))
  ;[1 1 1] Overlap Actor
  (if (`self.ActorHasTag` OtherActor "Player")
    (bind _returnvalue (`KismetSystemLibrary.K2_SetTimerDelegate` (delegate `DamageActor`) 0.5 true))
    (set `self.TimerHandle` _returnvalue)))

(event `DamageActor`
  ;[1 1 1] Damage Actor
  (`GameplayStatics.ApplyDamage` (stale `self.Box.OnComponentBeginOverlap` OtherActor) (`self.Damage`) null self))

(fn `UpdateWalkSpeed`
  (params (NewWalkSpeed :type "Float (double-precision)"))
  (set `CharacterMovementComponent.MaxWalkSpeed` NewWalkSpeed (`self.CharacterMovement`)))

(fn `UserConstructionScript`
  (`parent.UserConstructionScript`))