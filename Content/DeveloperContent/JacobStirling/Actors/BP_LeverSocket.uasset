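; BP_LeverSocket is an interactable socket that powers a connected lever with a charge carried by the player.
; Its Interaction event moves the charge from the player into an empty socket, or back from a filled socket to an empty-handed player.
; Each transfer updates the socket's HasCharge, the player's ChargeHeld and the lever's Active flag, then prints a status message.
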(event `/Game/DeveloperContent/JacobStirling/Management/BI_Interaction.Interaction`
  (params (PlayerCharacter :type "/Game/StarterStuff/FirstPerson/Blueprints/BP_FirstPersonCharacter Object Reference"))
  (bind _connectedlever (`self.ConnectedLever`))
  (bind _player_character (`self.Player Character`))
  (bind _hascharge (`self.HasCharge`))
  ;[1 1 1] Interaction Called
  (bind _output_get (set `self.Player Character` PlayerCharacter))
  (if (`/Game/StarterStuff/FirstPerson/Blueprints/BP_FirstPersonCharacter.ChargeHeld` _output_get)
    (if (not _hascharge)
      ;[1 1 1] Activate Lever
      (set `/Game/DeveloperContent/JacobStirling/Actors/BP_Lever.Active` true _connectedlever)
      (set `self.HasCharge` true)
      ;[1 1 1] Set player's charge
      (set `/Game/StarterStuff/FirstPerson/Blueprints/BP_FirstPersonCharacter.ChargeHeld` false _player_character)
      (`KismetSystemLibrary.PrintString` "I'm charged up!"))
    (elif _hascharge
      ;[1 1 1] Deactivate Lever
      (set `/Game/DeveloperContent/JacobStirling/Actors/BP_Lever.Active` false _connectedlever)
      (set `self.HasCharge` false)
      (set `/Game/StarterStuff/FirstPerson/Blueprints/BP_FirstPersonCharacter.ChargeHeld` true _player_character)
      (`KismetSystemLibrary.PrintString` "No Power"))))

(fn `UserConstructionScript`)