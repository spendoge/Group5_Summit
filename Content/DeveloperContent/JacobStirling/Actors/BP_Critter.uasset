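; BP_Critter is an interactable critter that the first-person player switches on and off by handing over or taking back a charge.
; On BeginPlay it caches the player as BP_FirstPersonCharacter.
; The Interaction event moves the charge by flipping the player's ChargeHeld flag and its own Active flag, activating only when the player holds a charge and deactivating only when they do not.
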(event `self.ReceiveBeginPlay`
  (bind _asbp_first_person_character (cast `/Game/StarterStuff/FirstPerson/Blueprints/BP_FirstPersonCharacter` (`GameplayStatics.GetPlayerCharacter` 0)))
  (set `self.As BP First Person Character` _asbp_first_person_character))

(event `/Game/DeveloperContent/JacobStirling/Management/BI_Interaction.Interaction`
  (params (PlayerCharacter :type "Actor Object Reference"))
  (bind _active (`self.Active`))
  (bind _as_bp_first_person_character (`self.As BP First Person Character`))
  ;[1 1 1] Call Interaction
  (if (`/Game/StarterStuff/FirstPerson/Blueprints/BP_FirstPersonCharacter.ChargeHeld` (`self.As BP First Person Character`))
    (if (not _active)
      ;[1 1 1] Set Critter Active
      (set `self.Active` true)
      ;[1 1 1] Set Player's Charge
      (set `/Game/StarterStuff/FirstPerson/Blueprints/BP_FirstPersonCharacter.ChargeHeld` false _as_bp_first_person_character))
    (elif _active
      (set `self.Active` false)
      (set `/Game/StarterStuff/FirstPerson/Blueprints/BP_FirstPersonCharacter.ChargeHeld` true _as_bp_first_person_character))))

(fn `UserConstructionScript`)