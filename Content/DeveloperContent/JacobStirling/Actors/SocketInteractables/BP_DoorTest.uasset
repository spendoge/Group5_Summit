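; Test door actor that slides open when activated through a socket or when all of its connected pressure plates or critters are triggered.
; Each bound handler removes triggered items from its array and re-adds released ones, independently calling Open when that array empties.
; Open plays a timeline that lerps the actor to EndLocation, with no closing logic.
; WirePowered follows the same pattern but is not bound here and has a hard-coded true condition.
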(event `self.ReceiveBeginPlay`
  ;[1 1 1] Bind event on begin play
  (add `/Game/DeveloperContent/JacobStirling/Actors/BP_PressurePlate.E_PressurePlateOverlapped` (`self.ConnectedPressurePlates`) (`|CreateDelegate` :!event `PressurePlateOverlapped`))
  (add `/Game/DeveloperContent/MilosDecermic/AI/baseCritter.E_Interacted` (`self.ConnectedCritters`) (`|CreateDelegate` :!event `CritterActivated`)))

(event `/Game/DeveloperContent/JacobStirling/Management/BI_SocketConnectors.Activate`
  (params (ActivityStatus :type Boolean))
  ;[1 1 1] Open door when socket is connected
  (if ActivityStatus
    (`self.Open`)))

(event `Open`
  ;[1 1 1] Move door to specified location
  (set `self.StartLocation` (`self.K2_GetActorLocation`))
  (bind (_direction _alpha) (`Timeline|T_OpenDoor` :!via `PlayFromStart`)
    (:`Update`
      (`self.K2_SetActorLocation` (`KismetMathLibrary.VLerp` (`self.StartLocation`) (`self.EndLocation`) _alpha)))))

(fn `CritterActivated`
  (params (Critter :type "/Game/DeveloperContent/MilosDecermic/AI/baseCritter Object Reference"))
  (bind _connectedcritters (`self.ConnectedCritters`))
  (bind _returnvalue (`KismetArrayLibrary.Array_Length` _connectedcritters))
  ;[1 1 1] Add and remove from the array based on critters' status
  (if (`/Game/DeveloperContent/MilosDecermic/AI/baseCritter.Active` Critter)
    (`KismetArrayLibrary.Array_RemoveItem` _connectedcritters Critter)
    (if (<= _returnvalue 0)
      (`self.Open`)
      (else
        (`KismetSystemLibrary.PrintString` (`KismetStringLibrary.Concat_StrStr` (`KismetStringLibrary.Conv_IntToString` _returnvalue) "remaining") :!label _label)))
    (else
      (`KismetArrayLibrary.Array_Add` (`self.ConnectedCritters`) Critter)
      (goto _label))))

(fn `PressurePlateOverlapped`
  (params (PressurePlate :type "/Game/DeveloperContent/JacobStirling/Actors/BP_PressurePlate Object Reference"))
  (bind _connectedpressureplates (`self.ConnectedPressurePlates`))
  ;[1 1 1] Add and remove from the array based on pressure plates' status
  (if (`/Game/DeveloperContent/JacobStirling/Actors/BP_PressurePlate.Overlapped` PressurePlate)
    (`KismetArrayLibrary.Array_RemoveItem` _connectedpressureplates PressurePlate)
    (if (<= (`KismetArrayLibrary.Array_Length` _connectedpressureplates) 0)
      (`self.Open`))
    (else
      (`KismetArrayLibrary.Array_Add` (`self.ConnectedPressurePlates`) PressurePlate))))

(fn `UserConstructionScript`
  (`parent.UserConstructionScript`))

(fn `WirePowered`
  (params (Wire :type "/Game/DeveloperContent/CamiToye/Wires/EndPower Object Reference"))
  (bind _connectedwires (`self.ConnectedWires`))
  ;[1 1 1] Add and Remove wires from the array based on their powered status
  (if true
    (`KismetArrayLibrary.Array_RemoveItem` _connectedwires Wire)
    (if (<= (`KismetArrayLibrary.Array_Length` _connectedwires) 0)
      (`self.Open`))
    (else
      (`KismetArrayLibrary.Array_Add` (`self.ConnectedWires`) Wire))))