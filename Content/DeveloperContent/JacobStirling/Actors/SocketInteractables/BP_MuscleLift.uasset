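; BP_MuscleLift is a socket-interactable lift whose platform moves when activated and returns when deactivated.
; BeginPlay caches the platform's world position as StartLocation, and a timeline lerps it toward EndLocation.
; Activate plays the timeline if the passed status is true, while Deactivate reverses it from its current point.
; SetMesh then swaps the platform material between powered and unpowered to match the Active state.
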(event `MovePlatform`
  ;[1 1 1] Platform Movement
  (bind (_direction _alpha) (`Timeline|T_PlatformMovement` :!label _label)
    (:`Update`
      (`SceneComponent.K2_SetWorldLocation` (`self.SM_MovingPlatform`) (`KismetMathLibrary.VLerp` (`self.StartLocation`) (`self.EndLocation`) _alpha) false false))))

(event `DontMovePlatform`
  ;[1 1 1] Platform Movement
  (goto _label :!via `Reverse`))

(event `self.ReceiveBeginPlay`
  ;[1 1 1] Set Start Location
  (set `self.StartLocation` (`SceneComponent.K2_GetComponentLocation` (`self.SM_MovingPlatform`))))

(event `/Game/DeveloperContent/JacobStirling/Management/BI_SocketConnectors.Activate`
  (params (ActivityStatus :type Boolean))
  ;[1 1 1] Set Activity
  (bind _output_get (set `self.Active` ActivityStatus))
  (if _output_get
    (`self.MovePlatform`)
    (`self.SetMesh` :!label _label_2)))

(event `/Game/DeveloperContent/JacobStirling/Management/BI_SocketConnectors.Deactivate`
  ;[1 1 1] Set Activity
  (set `self.Active` false)
  (`self.DontMovePlatform`)
  (goto _label_2))

(fn `SetMesh`
  (bind _sm_movingplatform (`self.SM_MovingPlatform`))
  (if (`self.Active`)
    (`PrimitiveComponent.SetMaterial` _sm_movingplatform 0 "/Game/DeveloperContent/SpencerWright/Master_Materials/MI_TestPowered.MI_TestPowered")
    (else
      (`PrimitiveComponent.SetMaterial` _sm_movingplatform 0 "/Game/DeveloperContent/SpencerWright/Master_Materials/MI_TestUnpowered.MI_TestUnpowered"))))

(fn `UserConstructionScript`
  (`parent.UserConstructionScript`))