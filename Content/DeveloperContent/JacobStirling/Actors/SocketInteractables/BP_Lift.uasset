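; BP_Lift is a powered lift platform that carries the player to a destination chosen by its charge level.
; Activate picks the destination from DesiredDestinations by charge level, and both Activate and Deactivate swap the platform's powered or unpowered material.
; While active, a Player-tagged actor entering the box plays a timeline that lerps the platform from its BeginPlay location, and leaving reverses it.
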(event `MovePlatform`
  ;[1 1 1] Platform Movement
  (bind (_direction _alpha) (`Timeline|T_PlatformMovement` :!via `PlayFromStart` :!label _label)
    (:`Update`
      (set `self.Alpha` _alpha)
      (`SceneComponent.K2_SetWorldLocation` (`self.SM_MovingPlatform`) (`KismetMathLibrary.VLerp` (`self.StartLocation`) (`self.Destination`) _alpha) false false))))

(event `StopMoving`
  ;[1 1 1] Platform Movement
  (goto _label :!via `Reverse`))

(event `self.ReceiveBeginPlay`
  ;[1 1 1] Set Start Location
  (set `self.StartLocation` (`SceneComponent.K2_GetComponentLocation` (`self.SM_MovingPlatform`))))

(event `/Game/DeveloperContent/JacobStirling/Management/BI_SocketConnectors.Activate`
  (params (ActivityStatus :type Boolean) (chargeLevel :type Integer))
  ;[1 1 1] Set Activity
  (bind _output_get (set `self.Charge Level` chargeLevel))
  (bind _output_get_2 (set `self.Active` ActivityStatus))
  (if _output_get_2
    (`self.SetLiftDestination` _output_get)
    (`self.SetMesh` :!label _label_2)))

(event `/Game/DeveloperContent/JacobStirling/Management/BI_SocketConnectors.Deactivate`
  (params (chargeLevel :type Integer))
  ;[1 1 1] Set Activity
  (set `self.Charge Level` chargeLevel)
  (set `self.Active` false)
  (goto _label_2))

(event `self.Box.OnComponentBeginOverlap`
  (params (OverlappedComponent :type "PrimitiveComponent Object Reference") (OtherActor :type "Actor Object Reference") (OtherComp :type "PrimitiveComponent Object Reference") (OtherBodyIndex :type Integer) (bFromSweep :type Boolean) (SweepResult :type "HitResult Structure (by ref)"))
  ;[1 1 1] Overlapped Actor
  (if (and (`self.Active`) (`self.ActorHasTag` OtherActor "Player"))
    (`self.MovePlatform`)))

(event `self.Box.OnComponentEndOverlap`
  (params (OverlappedComponent :type "PrimitiveComponent Object Reference") (OtherActor :type "Actor Object Reference") (OtherComp :type "PrimitiveComponent Object Reference") (OtherBodyIndex :type Integer))
  ;[1 1 1] Overlapped Actor
  (if (and (`self.Active`) (`self.ActorHasTag` OtherActor "Player"))
    (`self.StopMoving`)))

(fn `SetLiftDestination`
  (params (ChargeLevel :type Integer))
  (`KismetSystemLibrary.PrintString` (`KismetStringLibrary.Conv_IntToString` ChargeLevel))
  (set `self.Destination` (`|GetArrayItem` (`self.DesiredDestinations`) ChargeLevel)))

(fn `SetMesh`
  (bind _sm_movingplatform (`self.SM_MovingPlatform`))
  (if (`self.Active`)
    (`PrimitiveComponent.SetMaterial` _sm_movingplatform 0 "/Game/DeveloperContent/SpencerWright/Master_Materials/MI_TestPowered.MI_TestPowered")
    (else
      (`PrimitiveComponent.SetMaterial` _sm_movingplatform 0 "/Game/DeveloperContent/SpencerWright/Master_Materials/MI_TestUnpowered.MI_TestUnpowered"))))

(fn `UserConstructionScript`
  (`parent.UserConstructionScript`))