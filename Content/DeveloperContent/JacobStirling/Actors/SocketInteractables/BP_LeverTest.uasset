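; BP_LeverTest is a test lever actor that opens a connected actor, noted as a door, when used while powered.
; The Activate event sets the Powered flag from the status passed to it.
; The Interaction event checks that flag, calling Open on ConnectedActor if powered and otherwise only printing a deactivated debug message.
; It has no close or toggle logic.
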(event `/Game/DeveloperContent/JacobStirling/Management/BI_Interaction.Interaction`
  (params (PlayerCharacter :type "/Game/StarterStuff/FirstPerson/Blueprints/BP_FirstPersonCharacter Object Reference"))
  ;[1 1 1] Open door if powered
  (if (`self.Powered`)
    (`KismetSystemLibrary.PrintString` "Lever Activated")
    (`/Game/DeveloperContent/JacobStirling/Actors/SocketInteractables/BP_DoorTest.Open` (`self.ConnectedActor`))
    (else
      (`KismetSystemLibrary.PrintString` "Lever Deactivated"))))

(event `/Game/DeveloperContent/JacobStirling/Management/BI_SocketConnectors.Activate`
  (params (ActivityStatus :type Boolean))
  ;[1 1 1] Set Powered status
  (set `self.Powered` ActivityStatus))

(fn `UserConstructionScript`
  (`parent.UserConstructionScript`))