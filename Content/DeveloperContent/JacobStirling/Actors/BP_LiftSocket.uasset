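; Power socket that takes charge from the player on interaction to drive a connected lift.
; Each charge given raises the socket's level up to a maximum, activates the lift at that level and plays a sound pitched by it.
; SetMesh swaps the powered or unpowered material, starting from the Powered flag at BeginPlay.
; Logic for returning charge and deactivating the lift is left unwired; a full socket only decrements its count and calls SetChargeLevel(false).
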(event `self.ReceiveBeginPlay`
  ;[1 1 1] Set Activity Status on begin play
  (`self.SetMesh`)
  (if (`self.Powered`)
    (set `self.currentCharge` 1)
    (else
      (set `self.currentCharge` 0))))

(event `/Game/DeveloperContent/JacobStirling/Management/BI_Interaction.Interaction`
  (params (PlayerCharacter :type "/Game/StarterStuff/FirstPerson/Blueprints/BP_FirstPersonCharacter Object Reference"))
  (bind _currentcharge (`self.currentCharge`))
  (bind _player_character (`self.Player Character`))
  (bind _currentcharge_2 (`self.currentCharge`))
  ;[1 1 1] Check player charge level
  (bind _output_get (set `self.Player Character` PlayerCharacter))
  (if (>= (`/Game/StarterStuff/FirstPerson/Blueprints/BP_FirstPersonCharacter.ChargeLevel` _output_get) 1.0)
    (if (or (and (< _currentcharge (`self.maxCharge`)) (!= _currentcharge 0)) (== (`self.currentCharge`) 0))
      ;[1 1 1] Give charge to socket, take 1 from player
      (`/Engine/EditorBlueprintResources/StandardMacros.IncrementInt` (`self.currentCharge`)
        (:`  `
          (`/Game/StarterStuff/FirstPerson/Blueprints/BP_FirstPersonCharacter.SetChargeLevel` (`self.Player Character`) false)
          (set `self.Powered` true)
          (`self.SetMesh`)
          (`/Game/DeveloperContent/JacobStirling/Actors/SocketInteractables/BP_MuscleLift.Activate Lift` (`self.ConnectedLift`) true _currentcharge_2)
          (`KismetSystemLibrary.PrintString` (`KismetStringLibrary.Conv_IntToString` _currentcharge_2))
          (`GameplayStatics.PlaySoundAtLocation` "/Game/Audio/puzzleComplete.puzzleComplete" (`self.K2_GetActorLocation` self) (struct) 1.0 (`KismetMathLibrary.Conv_IntToDouble` _currentcharge_2) 0.0 null null null null)))
      (elif (< (`/Game/StarterStuff/FirstPerson/Blueprints/BP_FirstPersonCharacter.ChargeLevel` _player_character) (`/Game/StarterStuff/FirstPerson/Blueprints/BP_FirstPersonCharacter.maxCharge` _player_character))
        (set `self.IncreaseCharge?` false)
        (`/Engine/EditorBlueprintResources/StandardMacros.DecrementInt` (`self.currentCharge`)
          (:`  `
            (`/Game/StarterStuff/FirstPerson/Blueprints/BP_FirstPersonCharacter.SetChargeLevel` (`self.Player Character`) false)))))))

(fn `SetMesh`
  (bind _staticmesh (`self.StaticMesh`))
  (if (`self.Powered`)
    (`PrimitiveComponent.SetMaterial` _staticmesh 0 "/Game/DeveloperContent/SpencerWright/Master_Materials/MI_TestPowered.MI_TestPowered")
    (else
      (`PrimitiveComponent.SetMaterial` _staticmesh 0 "/Game/DeveloperContent/SpencerWright/Master_Materials/MI_TestUnpowered.MI_TestUnpowered"))))

(fn `UserConstructionScript`)