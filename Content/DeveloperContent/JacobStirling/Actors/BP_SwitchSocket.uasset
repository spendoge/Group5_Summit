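; BP_SwitchSocket is an interactable socket that takes a charge carried by the player to power a connected switch.
; On BeginPlay it caches the first-person player character.
; On Interaction, a player holding a charge fills an empty socket and activates ConnectedSwitch, while an empty-handed player takes the charge back and deactivates it.
; The charge moves between the socket's HasCharge and the character's ChargeHeld booleans.
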(event `self.ReceiveBeginPlay`
  ;[1 1 1] Cast to First Person Character
  (bind _asbp_first_person_character (cast `/Game/StarterStuff/FirstPerson/Blueprints/BP_FirstPersonCharacter` (`GameplayStatics.GetPlayerCharacter` 0)))
  (set `self.As BP First Person Character` _asbp_first_person_character))

(event `/Game/DeveloperContent/JacobStirling/Management/BI_Interaction.Interaction`
  (params (PlayerCharacter :type "Actor Object Reference"))
  (bind _connectedswitch (`self.ConnectedSwitch`))
  (bind _as_bp_first_person_character (`self.As BP First Person Character`))
  (bind _hascharge (`self.HasCharge`))
  ;[1 1 1] Interaction Called
  (if (`/Game/StarterStuff/FirstPerson/Blueprints/BP_FirstPersonCharacter.ChargeHeld` (`self.As BP First Person Character`))
    (if (not _hascharge)
      ;[1 1 1] Activate Switch
      (set `/Game/DeveloperContent/JacobStirling/Actors/BP_Switch.Active` true _connectedswitch)
      (set `self.HasCharge` true)
      ;[1 1 1] Set player's charge
      (set `/Game/StarterStuff/FirstPerson/Blueprints/BP_FirstPersonCharacter.ChargeHeld` false _as_bp_first_person_character))
    (elif _hascharge
      ;[1 1 1] Deactivate Switch
      (set `/Game/DeveloperContent/JacobStirling/Actors/BP_Switch.Active` false _connectedswitch)
      (set `self.HasCharge` false)
      (set `/Game/StarterStuff/FirstPerson/Blueprints/BP_FirstPersonCharacter.ChargeHeld` true _as_bp_first_person_character))))

(fn `UserConstructionScript`)