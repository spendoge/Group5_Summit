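; BP_PressurePlateDoor is a door actor that opens once all of its connected pressure plates are pressed.
; On BeginPlay it binds to the overlap event of the plates in ConnectedPressurePlates.
; A pressed plate leaves the array and a released one rejoins it, with the remaining count printed on screen.
; When the array empties, a timeline lerps the door from its current location to EndLocation.
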(event `PressurePlateOverlapped`
  (params (PressurePlate :type "/Game/DeveloperContent/JacobStirling/Actors/BP_PressurePlate Object Reference"))
  (bind _connectedpressureplates (`self.ConnectedPressurePlates`))
  (bind _returnvalue (`KismetArrayLibrary.Array_Length` _connectedpressureplates))
  ;[1 1 1] Add and remove actors from array
  (if (`/Game/DeveloperContent/JacobStirling/Actors/BP_PressurePlate.Overlapped` PressurePlate)
    (`KismetArrayLibrary.Array_RemoveItem` _connectedpressureplates PressurePlate)
    (if (<= _returnvalue 0)
      (`self.Open`)
      (else
        (`KismetSystemLibrary.PrintString` (`KismetStringLibrary.Concat_StrStr` (`KismetStringLibrary.Conv_IntToString` _returnvalue) "remaining") :!label _label)))
    (else
      (`KismetArrayLibrary.Array_Add` (`self.ConnectedPressurePlates`) PressurePlate)
      (goto _label))))

(event `self.ReceiveBeginPlay`
  ;[1 1 1] Bind event
  (add `/Game/DeveloperContent/JacobStirling/Actors/BP_PressurePlate.E_PressurePlateOverlapped` (`self.ConnectedPressurePlates`) (`|CreateDelegate` :!event `PressurePlateOverlapped`)))

(event `Open`
  ;[1 1 1] Open Door
  (set `self.StartLocation` (`self.K2_GetActorLocation`))
  (bind (_direction _alpha) (`Timeline|T_OpenDoor` :!via `PlayFromStart`)
    (:`Update`
      (`self.K2_SetActorLocation` (`KismetMathLibrary.VLerp` (`self.StartLocation`) (`self.EndLocation`) _alpha)))))

(fn `UserConstructionScript`)