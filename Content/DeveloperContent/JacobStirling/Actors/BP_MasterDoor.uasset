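; BP_MasterDoor is a door actor that opens once all of its connected wires are activated.
; WireActivated removes each activated wire from ConnectedWires and calls Open when none remain.
; Open records the current location and plays a timeline that lerps the actor to EndLocation without sweeping.
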(event `Open`
  ;[1 1 1] Open Door
  (set `self.StartLocation` (`self.K2_GetActorLocation`))
  (bind (_direction _alpha) (`Timeline|T_OpenDoor` :!via `PlayFromStart`)
    (:`Update`
      (`self.K2_SetActorLocation` (`KismetMathLibrary.VLerp` (`self.StartLocation`) (`self.EndLocation`) _alpha)))))

(fn `UserConstructionScript`)

(fn `WireActivated`
  (params (WIres :type "/Game/DeveloperContent/CamiToye/Wires/EndPower Object Reference"))
  (bind _connectedwires (`self.ConnectedWires`))
  ;[1 1 1] Remove Wires from the array when they're activated
  (`KismetArrayLibrary.Array_RemoveItem` _connectedwires WIres)
  (if (<= (`KismetArrayLibrary.Array_Length` _connectedwires) 0)
    (`self.Open`)))