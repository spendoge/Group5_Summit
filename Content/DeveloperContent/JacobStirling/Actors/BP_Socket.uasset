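; Interactable power socket that takes a charge from the player or gives it back, powering linked actors.
; Interaction toggles Powered from the socket and player charge states, updates the player, and sends activate or deactivate messages to every ConnectedActor.
; BeginPlay sends the initial state to linked actors and ConnectedWire.
; SetPower clears Powered on master-door unlock without notifying them, and SetMesh picks the powered or unpowered material.
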(event `/Game/DeveloperContent/JacobStirling/Management/BI_Interaction.Interaction`
  (params (PlayerCharacter :type "/Game/StarterStuff/FirstPerson/Blueprints/BP_FirstPersonCharacter Object Reference"))
  (bind _powered (`self.Powered`))
  (bind _connectedactor (`self.ConnectedActor`))
  ;[1 1 1] Interaction Called
  (bind _output_get (set `self.Player Character` PlayerCharacter))
  (if (`/Game/StarterStuff/FirstPerson/Blueprints/BP_FirstPersonCharacter.ChargeHeld` _output_get)
    (if (not _powered)
      (set `self.Powered` true)
      ;[1 1 1] Set Player's Charge
      (`/Game/StarterStuff/FirstPerson/Blueprints/BP_FirstPersonCharacter.SetCharge` (`self.Player Character`) false)
      (for _array_element _connectedactor
        (message `/Game/DeveloperContent/JacobStirling/Management/BI_SocketConnectors.Activate` _array_element true)))
    (elif _powered
      (set `self.Powered` false)
      (`/Game/StarterStuff/FirstPerson/Blueprints/BP_FirstPersonCharacter.SetCharge` (`self.Player Character`) true)
      (for _array_element_2 _connectedactor
        (message `/Game/DeveloperContent/JacobStirling/Management/BI_SocketConnectors.Deactivate` _array_element_2)))))

(event `self.ReceiveBeginPlay`
  (bind _powered (`self.Powered`))
  ;[1 1 1] Set Activity Status on begin play
  (for _array_element (`self.ConnectedActor`)
    (message `/Game/DeveloperContent/JacobStirling/Management/BI_SocketConnectors.Activate` _array_element _powered)
    (message `/Game/DeveloperContent/JacobStirling/Management/BI_SocketConnectors.Activate` (`self.ConnectedWire`) _powered)))

(event `SetPower`
  ;[1 1 1] Deactivate when master door unlocked
  (set `self.Powered` false))

(fn `SetMesh`
  (bind _staticmesh (`self.StaticMesh`))
  (if (`self.Powered`)
    (`PrimitiveComponent.SetMaterial` _staticmesh 0 "/Game/DeveloperContent/SpencerWright/Master_Materials/MI_TestPowered.MI_TestPowered")
    (else
      (`PrimitiveComponent.SetMaterial` _staticmesh 0 "/Game/DeveloperContent/SpencerWright/Master_Materials/MI_TestUnpowered.MI_TestUnpowered"))))

(fn `UserConstructionScript`)