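; BP_WBCAIController is an AI controller that runs the BT_WBC behavior tree on possession and tracks whether the player is perceived.
; A successful perception update for a "Player"-tagged actor cancels the timer, sets LineOfSight and writes that actor into the SelfActor blackboard key.
; Any other perception update starts a one-shot grace timer of LineOfSightTimer length, which clears both keys when it expires.
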(event `self.ReceivePossess`
  (params (PossessedPawn :type "Pawn Object Reference"))
  ;[1 1 1] Run Behaviour Tree on possession
  (`KismetSystemLibrary.PrintString` "AI Running")
  (`self.RunBehaviorTree` "/Game/DeveloperContent/JacobStirling/Actors/AI/BT_WBC.BT_WBC"))

(event `self.AIPerception.OnTargetPerceptionUpdated`
  (params (Actor :type "Actor Object Reference") (Stimulus :type "AIStimulus Structure"))
  (bind _blackboard (`self.Blackboard`))
  ;[1 1 1] Update Line of Sight if Player has been detected
  (if (and (`self.ActorHasTag` Actor "Player") (`.bSuccessfullySensed` (break `AIStimulus` Stimulus)))
    (`KismetSystemLibrary.K2_ClearAndInvalidateTimerHandle` (`self.WBCTimer`))
    (`BlackboardComponent.SetValueAsBool` _blackboard "LineOfSight" true)
    (`BlackboardComponent.SetValueAsObject` _blackboard "SelfActor" Actor)
    (else
      (bind _returnvalue (`KismetSystemLibrary.K2_SetTimerDelegate` (delegate `StartWBCTimer`) (`self.LineOfSightTimer`)))
      (set `self.WBCTimer` _returnvalue))))

(event `StartWBCTimer`
  (bind _blackboard (`self.Blackboard`))
  ;[1 1 1] Start timer for Line of Sight update
  (`BlackboardComponent.SetValueAsBool` _blackboard "LineOfSight" false)
  (`BlackboardComponent.SetValueAsObject` _blackboard "SelfActor" null))

(fn `UserConstructionScript`)