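; BP_ButtonSocket is an interactable charge socket that switches its connected button on and off.
; On BeginPlay it caches the player's BP_FirstPersonCharacter, whose ChargeHeld flag is read on each Interaction event.
; Interacting while holding a charge activates the button if the socket is empty; interacting without one deactivates it if filled.
; It tracks its own HasCharge state but never changes the character's ChargeHeld flag.
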(event `self.ReceiveBeginPlay`
  ;[1 1 1] Cast to First Person Character
  (bind _asbp_first_person_character (cast `/Game/StarterStuff/FirstPerson/Blueprints/BP_FirstPersonCharacter` (`GameplayStatics.GetPlayerCharacter` 0)))
  (set `self.As BP First Person Character` _asbp_first_person_character))

(event `/Game/DeveloperContent/JacobStirling/Management/BI_Interaction.Interaction`
  (bind _connectedbutton (`self.ConnectedButton`))
  (bind _hascharge (`self.HasCharge`))
  ;[1 1 1] Interaction Called
  (if (`/Game/StarterStuff/FirstPerson/Blueprints/BP_FirstPersonCharacter.ChargeHeld` (`self.As BP First Person Character`))
    (if (not _hascharge)
      ;[1 1 1] Activate button
      (`/Game/DeveloperContent/JacobStirling/Actors/BP_Button.Activate` _connectedbutton)
      (set `self.HasCharge` true))
    (elif _hascharge
      ;[1 1 1] Deactivate Button
      (`/Game/DeveloperContent/JacobStirling/Actors/BP_Button.Deactivate` _connectedbutton)
      (set `self.HasCharge` false))))

(fn `UserConstructionScript`)